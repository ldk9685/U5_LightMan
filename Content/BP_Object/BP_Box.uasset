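; BP_Box is a timed pad trigger that swaps a box and cube for a changed hole material.
; Overlapping Pad_Col starts a timer that Tick accumulates, and ending the overlap resets it.
; After two seconds MoveBox destroys the referenced CubeBP actor and the Box component, then applies M_Box to Hole, so nothing physically moves.
; The overlap does not filter which actor triggers it.
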(event OnComponentBeginOverlap(Pad_Col)
  (params (OverlappedComponent :type Primitive%20Component%20Object%20Reference) (OtherActor :type Actor%20Object%20Reference) (OtherComp :type Primitive%20Component%20Object%20Reference) (OtherBodyIndex :type Integer) (bFromSweep :type Boolean) (SweepResult :type Hit%20Result%20Structure%20%28by%20ref%29))
  (Variables|Default|SetIsStanding true)
  (Variables|Default|SetTimer 0.0))

(event OnComponentEndOverlap(Pad_Col)
  (params (OverlappedComponent :type Primitive%20Component%20Object%20Reference) (OtherActor :type Actor%20Object%20Reference) (OtherComp :type Primitive%20Component%20Object%20Reference) (OtherBodyIndex :type Integer))
  (Variables|Default|SetIsStanding false)
  (Variables|Default|SetTimer 0.0))

(event Custom|MoveBox
  (Actor|DestroyActor (Variables|Default|GetCubeBP))
  (Components|DestroyComponent (Variables|Default|GetBox))
  (Rendering|Material|SetMaterial (Variables|Default|GetHole) 0 "/Game/BP_Object/M_Box.M_Box"))

(event EventTick
  (params (DeltaSeconds :type Float%20%28single-precision%29))
  (if (== (Variables|Default|GetIsStanding) true)
    (Variables|Default|SetTimer (+ (Variables|Default|GetTimer) DeltaSeconds))
    (if (>= (Variables|Default|GetTimer) 2.0)
      (CallFunction|MoveBox)
      (Variables|Default|SetIsStanding false))))

(event Collision|EventActorBeginOverlap
  (params (OtherActor :type Actor%20Object%20Reference)))

(event EventBeginPlay)

(fn ConstructionScript)