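; Guard monster that chases the player on sight and shows the game-over UI when its capsule hits BP_TopDownCharacter.
; PawnSensing starts an AI move toward the player, and a one-second timer set at launch or on failure calls StopChase.
; StopChase clears the IsChasing flag, which blocks re-triggering, and moves the monster back to its BeginPlay position.
; Tick prints the flag for debugging.
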(event OnSeePawn(PawnSensing)
  (params (Pawn :type Pawn%20Object%20Reference))
  (if (== (Variables|Default|GetIsChasing) false)
    (Variables|Default|SetIsChasing true)
    (AI|AIMoveTo self "0, 0, 0" (Game|GetPlayerCharacter 0) 5.0 false
      (:then
        (Utilities|Time|SetTimerbyEvent (delegate Custom|StopChase) 1.0))
      (:OnFail
        (Utilities|Time|SetTimerbyEvent (delegate Custom|StopChase) 1.0)))))

(event OnComponentHit(CapsuleComponent)
  (params (HitComponent :type Primitive%20Component%20Object%20Reference) (OtherActor :type Actor%20Object%20Reference) (OtherComp :type Primitive%20Component%20Object%20Reference) (NormalImpulse :type Vector :default "0, 0, 0") (Hit :type Hit%20Result%20Structure%20%28by%20ref%29))
  (bind _asbp_top_down_character (Utilities|Casting|CastToBP_TopDownCharacter OtherActor))
  (Default|GameOverUI _asbp_top_down_character))

(event Custom|StopChase
  (Variables|Default|SetIsChasing false)
  (AI|AIMoveTo self (Variables|Default|GetStartPosition) 0 5.0 false))

(event EventBeginPlay
  (Variables|Default|SetStartPosition (Transformation|GetActorLocation))
  (Variables|Default|SetIsChasing false))

(event EventTick
  (params (DeltaSeconds :type Float%20%28single-precision%29))
  (Development|PrintString (Utilities|String|ToString(Boolean) (Variables|Default|GetIsChasing))))

(fn ConstructionScript)