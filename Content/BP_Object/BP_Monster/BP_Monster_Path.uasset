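; Patrolling monster that chases the player on sight and triggers the game-over UI when its capsule hits the player character.
; On BeginPlay it gathers four points from the linked BP_WayPoints actor and loops through them with chained AIMoveTo calls.
; PawnSensing switches it to chasing player 0, guarded by IsChasing.
; A three-second timer, started as the chase begins or if it fails, returns it to the current waypoint.
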(event OnSeePawn(PawnSensing)
  (params (Pawn :type Pawn%20Object%20Reference))
  (if (not (Variables|Default|GetIsChasing))
    (Variables|Default|SetIsChasing true)
    (AI|AIMoveTo self "0, 0, 0" (Game|GetPlayerCharacter 0) 5.0 false
      (:then
        (Utilities|Time|SetTimerbyEvent (delegate Custom|StopChase) 3.0))
      (:OnFail
        (Utilities|Time|SetTimerbyEvent (delegate Custom|StopChase) 3.0)))))

(event OnComponentHit(CapsuleComponent)
  (params (HitComponent :type Primitive%20Component%20Object%20Reference) (OtherActor :type Actor%20Object%20Reference) (OtherComp :type Primitive%20Component%20Object%20Reference) (NormalImpulse :type Vector :default "0, 0, 0") (Hit :type Hit%20Result%20Structure%20%28by%20ref%29))
  (bind _asbp_top_down_character (Utilities|Casting|CastToBP_TopDownCharacter OtherActor))
  (Default|GameOverUI _asbp_top_down_character))

(event Custom|MoveToNext
  (AI|AIMoveTo self (Transformation|GetWorldLocation (Utilities|Array|Get(acopy) (Variables|Default|GetWayArray) (Variables|Default|GetcurrentIndex))) 0 5.0 false
    (:OnSuccess
      (Variables|Default|SetcurrentIndex (+ (Variables|Default|GetcurrentIndex) 1))
      (if (>= (Variables|Default|GetcurrentIndex) (Utilities|Array|Length (Variables|Default|GetWayArray)))
        (Variables|Default|SetcurrentIndex 0)
        (CallFunction|MovetoNext)
        (else
          (CallFunction|MovetoNext))))))

(event Custom|StopChase
  (Variables|Default|SetIsChasing false)
  (CallFunction|MovetoNext))

(event EventBeginPlay
  (bind _wayarray (Variables|Default|GetWayArray))
  (Utilities|IsValid (Variables|Default|GetWayPointBP)
    (:Is%20Valid
      (bind _asbp_way_points (Utilities|Casting|CastToBP_WayPoints (Variables|Default|GetWayPointBP)))
      (Utilities|Array|Add _wayarray (Variables|/Game/BP_Object/BP_Monster/BP_WayPoints.BP_WayPoints_C|Getway1 _asbp_way_points))
      (Utilities|Array|Add _wayarray (Variables|/Game/BP_Object/BP_Monster/BP_WayPoints.BP_WayPoints_C|Getway2 _asbp_way_points))
      (Utilities|Array|Add _wayarray (Variables|/Game/BP_Object/BP_Monster/BP_WayPoints.BP_WayPoints_C|Getway3 _asbp_way_points))
      (Utilities|Array|Add _wayarray (Variables|/Game/BP_Object/BP_Monster/BP_WayPoints.BP_WayPoints_C|Getway4 _asbp_way_points))
      (CallFunction|MovetoNext))))

(event Collision|EventActorBeginOverlap
  (params (OtherActor :type Actor%20Object%20Reference)))

(event EventTick
  (params (DeltaSeconds :type Float%20%28single-precision%29)))

(fn ConstructionScript)